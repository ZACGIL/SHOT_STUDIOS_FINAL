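; Spawner Blueprint that places a health pickup in the world where the player left-clicks.
; On click, if HealthPickup passes its check, it deprojects the mouse position and line-traces on the Visibility channel out to Tracedistance, with debug drawing.
; The pickup spawns at the impact point, without checking whether the trace hit anything.
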(event `Key|LeftMouseButton`
  (params (Key :type "Key Structure"))
  (bind (_worldlocation _worlddirection) (`PlayerController.DeprojectMousePositionToWorld` (`GameplayStatics.GetPlayerController` 0)))
  (:`Pressed`
    (if (`self.HealthPickup`)
      (bind _outhit (`KismetSystemLibrary.LineTraceSingle` :`Start` _worldlocation :`End` (+ _worldlocation (* _worlddirection (`self.tracedistance`))) :`TraceChannel` "TraceTypeQuery1" :`DrawDebugType` "ForDuration"))
      (`|SpawnActorFromClass` "/Game/TopDownBP/HealthPickup.HealthPickup_C" (`KismetMathLibrary.Conv_VectorToTransform` (`.ImpactPoint` (`GameplayStatics.BreakHitResult` _outhit))) "Undefined" "OverrideRootScale" null null))))

(fn `UserConstructionScript`)