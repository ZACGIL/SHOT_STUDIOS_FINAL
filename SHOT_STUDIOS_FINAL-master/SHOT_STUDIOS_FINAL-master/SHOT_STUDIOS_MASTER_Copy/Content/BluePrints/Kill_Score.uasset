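; Kill score actor that shows the enemy kill count on its Score widget component and can persist it.
; BeginPlay caches the TopDownGameMode and the Score widget, then Tick pushes EnemiesDead to the widget's text every frame.
; SaveGame and LoadGame events write and restore the count through a MySaveGame object in a fixed slot.
; The cached game mode is unused here, and nothing in this graph increments the count.
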(event `self.ReceiveBeginPlay`
  (bind _outactors (`GameplayStatics.GetAllActorsOfClass` "/Game/TopDownBP/Blueprints/TopDownGameMode.TopDownGameMode_C"))
  (set `self.GameMode` (`|GetArrayItem` _outactors))
  (bind _asscore (cast `/Game/TopDownBP/Blueprints/Widgets/Score` (`WidgetComponent.GetUserWidgetObject` (`self.Widget`))))
  (set `self.ScoreBoard` _asscore))

(event `self.ReceiveTick`
  (params (DeltaSeconds :type "Float (single-precision)"))
  (bind _output_get (set `self.EnemiesDead` (`self.EnemiesDead`)))
  (set `/Game/TopDownBP/Blueprints/Widgets/Score.EnemiesKilled` (`KismetTextLibrary.Conv_IntToText` _output_get) (`self.ScoreBoard`)))

(event `SaveGame`
  (bind _saversubclass (`self.SaverSubClass`))
  (bind _returnvalue (`GameplayStatics.CreateSaveGameObject` "/Game/MySaveGame.MySaveGame_C"))
  (set `self.SaverSubClass` _returnvalue)
  (bind _asmy_save_game (cast `/Game/MySaveGame` _saversubclass))
  (set `/Game/MySaveGame.EnemiesKilled` (`self.EnemiesDead`) _asmy_save_game)
  (`GameplayStatics.SaveGameToSlot` _saversubclass (`self.SaveGame1FileSave`)))

(event `LoadGame`
  (bind _returnvalue (`GameplayStatics.LoadGameFromSlot` (`self.SaveGame1FileSave`)))
  (set `self.SaverSubClass` _returnvalue)
  (bind _asmy_save_game (cast `/Game/MySaveGame` (`self.SaverSubClass`)))
  (set `self.EnemiesDead` (`/Game/MySaveGame.EnemiesKilled` _asmy_save_game)))

(fn `UserConstructionScript`)