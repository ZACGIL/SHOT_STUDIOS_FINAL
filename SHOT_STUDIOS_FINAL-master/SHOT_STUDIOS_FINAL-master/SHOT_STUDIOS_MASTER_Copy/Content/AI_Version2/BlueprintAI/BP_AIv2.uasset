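; BP_AIv2 is a sword-wielding enemy AI character with walk and run speed events, a health bar widget refreshed every Tick, and a socket-attached sword.
; Any actor overlap makes it damage itself, crediting the first Halberd_A found; at zero health it increments Kill_Score's dead-enemy count and is destroyed.
; Attack plays a slash and opens a timed window in which capsule overlaps damage TopDownCharacter, then restores the animation Blueprint.
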(event `self.ReceiveBeginPlay`
  (bind _asnew_enemy_health_bar (cast `/Game/TopDownBP/Blueprints/Widgets/New_Enemy_HealthBar` (`WidgetComponent.GetUserWidgetObject` (`self.Widget`))))
  (bind _output_get (set `self.NewEnemyHealthBar` _asnew_enemy_health_bar))
  (set `/Game/TopDownBP/Blueprints/Widgets/New_Enemy_HealthBar.HBar` (/ (`self.HealthAI`) 100.0) _output_get))

(event `self.ReceiveActorBeginOverlap`
  (params (OtherActor :type "Actor Object Reference"))
  (bind _outactors (`GameplayStatics.GetAllActorsOfClass` "/Game/BluePrints/Halberd_A.Halberd_A_C"))
  (bind _output_get (set `self.Halberd` (`|GetArrayItem` _outactors)))
  (`GameplayStatics.ApplyDamage` self 10.0 null _output_get))

(event `self.ReceiveAnyDamage`
  (params (Damage :type "Float (single-precision)") (DamageType :type "DamageType Object Reference") (InstigatedBy :type "Controller Object Reference") (DamageCauser :type "Actor Object Reference"))
  (set `self.HealthAI` (- (`self.HealthAI`) Damage))
  (if (<= (`self.HealthAI`) 0.0)
    (bind _outactors (`GameplayStatics.GetAllActorsOfClass` "/Game/BluePrints/Kill_Score.Kill_Score_C"))
    (bind _output_get (set `self.Score` (`|GetArrayItem` _outactors)))
    (bind _result (`/Engine/EditorBlueprintResources/StandardMacros.IncrementInt` (`/Game/BluePrints/Kill_Score.EnemiesDead` _output_get))
      (:`  `
        (set `/Game/BluePrints/Kill_Score.EnemiesDead` _result _output_get)
        (`self.K2_DestroyActor`)))))

(event `self.ReceiveTick`
  (params (DeltaSeconds :type "Float (single-precision)"))
  (set `/Game/TopDownBP/Blueprints/Widgets/New_Enemy_HealthBar.HBar` (/ (`self.HealthAI`) 100.0) (`self.NewEnemyHealthBar`)))

(event `Walk`
  (set `CharacterMovementComponent.MaxWalkSpeed` 250.0 (`self.CharacterMovement`)))

(event `Run`
  (set `CharacterMovementComponent.MaxWalkSpeed` 460.0 (`self.CharacterMovement`)))

(event `Attack`
  (`SkeletalMeshComponent.PlayAnimation` (`self.Mesh`) "/Game/AI_Version2/BlueprintAI/Anim/Stable_Sword_Inward_Slash.Stable_Sword_Inward_Slash" false)
  (set `self.Attacking` true)
  (`KismetSystemLibrary.Delay` 1.5)
  (set `self.Attacking` false)
  (`SkeletalMeshComponent.SetAnimationMode` (`self.Mesh`) "AnimationBlueprint"))

(event `self.Capsule.OnComponentBeginOverlap`
  (params (OverlappedComponent :type "PrimitiveComponent Object Reference") (OtherActor :type "Actor Object Reference") (OtherComp :type "PrimitiveComponent Object Reference") (OtherBodyIndex :type Integer) (bFromSweep :type Boolean) (SweepResult :type "HitResult Structure (by ref)"))
  (if (`self.Attacking`)
    (bind _astop_down_character (cast `/Game/TopDownBP/Blueprints/TopDownCharacter` OtherActor))
    (`/Game/TopDownBP/Blueprints/TopDownCharacter.Take Damage` _astop_down_character)))

(fn `UserConstructionScript`
  (`SceneComponent.K2_AttachToComponent` (`self.Sword`) (`self.Mesh`) "Sword" "KeepRelative" "KeepRelative" "KeepRelative" true))